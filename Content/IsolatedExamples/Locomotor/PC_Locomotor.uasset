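; Player controller for the Locomotor example that turns Enhanced Input actions into pawn movement and camera rotation.
; Move input is normalized and applied along the control rotation's right and forward vectors.
; Mouse look adds scaled-down yaw and pitch, with a note that the speed must match the control rig, while gamepad look scales by frame delta time.
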(event `EnhancedInput|/Game/Input/IA_Move`
  (params (ActionValue :type "Vector2D Structure") (ElapsedSeconds :type "Float (double-precision)") (TriggeredSeconds :type "Float (double-precision)") (InputAction :type "InputAction Object Reference" :default "/Game/Input/IA_Move.IA_Move"))
  (bind _returnvalue (`self.K2_GetPawn`))
  (bind _returnvalue_2 (`self.GetControlRotation`))
  (bind (_returnvalue_x _returnvalue_y) (`KismetMathLibrary.BreakVector2D` (`KismetMathLibrary.Normal2D` ActionValue)))
  (:`Triggered`
    (`Pawn.AddMovementInput` _returnvalue (`KismetMathLibrary.GetRightVector` _returnvalue_2) _returnvalue_x false)
    (`Pawn.AddMovementInput` _returnvalue (`KismetMathLibrary.GetForwardVector` _returnvalue_2) _returnvalue_y false)))

(event `EnhancedInput|/Game/Input/IA_Look`
  (params (ActionValue :type "Vector2D Structure") (ElapsedSeconds :type "Float (double-precision)") (TriggeredSeconds :type "Float (double-precision)") (InputAction :type "InputAction Object Reference" :default "/Game/Input/IA_Look.IA_Look"))
  (:`Triggered`
    (`self.AddYawInput` (/ ActionValue_X 15.0))
    (`self.AddPitchInput` (/ ActionValue_Y 15.0))))

(event `EnhancedInput|/Game/Input/IA_Look_Gamepad`
  (params (ActionValue :type "Vector2D Structure") (ElapsedSeconds :type "Float (double-precision)") (TriggeredSeconds :type "Float (double-precision)") (InputAction :type "InputAction Object Reference" :default "/Game/Input/IA_Look_Gamepad.IA_Look_Gamepad"))
  (bind (_returnvalue_x _returnvalue_y) (`KismetMathLibrary.BreakVector2D` (* ActionValue (`GameplayStatics.GetWorldDeltaSeconds`))))
  (:`Triggered`
    (`self.AddYawInput` _returnvalue_x)
    (`self.AddPitchInput` _returnvalue_y)))

(fn `UserConstructionScript`)