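; Player controller for the LookAtPOI example level that drives a selected zone character's look-at and switches between spectator and playable modes.
; Zone selection caches the pawn, gizmo and AnimInstance, enables look-at and updates the GUI widget.
; Tick feeds the AnimBP a target: a gizmo-relative point, or the player's head socket while playing.
; Spawning possesses a Mover character and destroys gizmos; spectator mode removes it and deselects zones.
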(event `self.ReceiveBeginPlay`
  (set `PlayerCameraManager.DefaultFOV` 32.0 (`self.PlayerCameraManager`))
  ; Spawn Widget
  (bind _returnvalue (`|CreateWidget` "/Game/IsolatedExamples/LookAtPOI/TestLevelContent/Widget/WB_LookAtPOI__GUI.WB_LookAtPOI__GUI_C" self))
  (`UserWidget.AddToViewport` _returnvalue 0)
  (set `self.Level Widget` _returnvalue))

(event `self.ReceiveTick`
  (params (DeltaSeconds :type "Float (single-precision)"))
  (if (`self.Look At Enabled`)
    (`self.Set Look At Target On Anim Instance`)))

(event `Zone Was Selected`
  (params (`Active  Pawn` :type "Pawn Object Reference") (Type :type String) (`Gizmo Onj` :type "/Game/IsolatedExamples/LookAtPOI/TestLevelContent/Props/BP_LookAtPOI_TargetGizmo Object Reference"))
  (set `self.Selected Zone Type` Type)
  (bind _aspawn_look_at_poi_char (cast `/Game/IsolatedExamples/LookAtPOI/TestLevelContent/Characters/Pawn_LookAt_POI_Char` `Active  Pawn`))
  (bind _output_get (set `self.Active Pawn` _aspawn_look_at_poi_char))
  (set `self.Gizmo Obj` `Gizmo Onj`)
  (set `self.AnimInstance` (`SkeletalMeshComponent.GetAnimInstance` (`self.GetComponentByClass` _output_get "/Script/Engine.SkeletalMeshComponent")))
  (set `self.Look At Enabled` true)
  (`self.Set Look At Target On Anim Instance`)
  (bind _asabp_look_at_poi_char (cast `/Game/IsolatedExamples/LookAtPOI/TestLevelContent/Characters/ABP_LookAtPOI_Char` (`self.AnimInstance`)))
  (set `/Game/IsolatedExamples/LookAtPOI/TestLevelContent/Characters/ABP_LookAtPOI_Char.LookAtPOI Enabled` true _asabp_look_at_poi_char)
  (`/Game/IsolatedExamples/LookAtPOI/TestLevelContent/Widget/WB_LookAtPOI__GUI.Zone Selected` (`self.Level Widget`) (`self.Selected Zone Type`) _asabp_look_at_poi_char))

(event `Play Gesture Montage`
  (params (Montage :type "AnimMontage Object Reference"))
  (`AnimInstance.Montage_Play` (`self.AnimInstance`) Montage 1.0 "MontageLength" 0.0 true))

(event `Spawn Player`
  (bind _returnvalue (`|SpawnActorFromClass` "/Game/Blueprints/SandboxCharacter_Mover.SandboxCharacter_Mover_C" (`KismetMathLibrary.MakeTransform` (0.0 0.0 100.0)) "Undefined" "MultiplyWithRoot" null null))
  (bind _output_get (set `self.Player Pawn` _returnvalue))
  (`self.Possess` self _output_get)
  (set `self.Look At Player` true)
  (bind _outactors (`GameplayStatics.GetAllActorsOfClass` "/Game/IsolatedExamples/LookAtPOI/TestLevelContent/Props/BP_LookAtPOI_BorderObj.BP_LookAtPOI_BorderObj_C"))
  (for _array_element _outactors
    (bind _gizmo_obj (`/Game/IsolatedExamples/LookAtPOI/TestLevelContent/Props/BP_LookAtPOI_BorderObj.Gizmo Obj` _array_element))
    (`/Engine/EditorBlueprintResources/StandardMacros.IsValid` _gizmo_obj
      (:`Is Valid`
        (`self.K2_DestroyActor` _gizmo_obj)))))

(event `Spectator Mode`
  (`self.UnPossess` self)
  (set `self.Look At Player` false)
  (set `self.Look At Enabled` false)
  (`self.K2_DestroyActor` (`self.Player Pawn`))
  (bind _outactors (`GameplayStatics.GetAllActorsOfClass` "/Script/Engine.SpectatorPawn"))
  (`self.Possess` self (`|GetArrayItem` _outactors))
  (bind _outactors_2 (`GameplayStatics.GetAllActorsOfClass` "/Game/IsolatedExamples/LookAtPOI/TestLevelContent/Props/BP_LookAtPOI_BorderObj.BP_LookAtPOI_BorderObj_C"))
  (for _array_element _outactors_2
    (`/Game/IsolatedExamples/LookAtPOI/TestLevelContent/Props/BP_LookAtPOI_BorderObj.Deselect Zone` _array_element)))

(fn `Set Look At Target On Anim Instance`
  (bind _gizmo_obj (`self.Gizmo Obj`))
  (bind _returnvalue_x (`KismetMathLibrary.BreakVector` (`self.GetActorScale3D` _gizmo_obj)))
  (if true
    (if (`self.Look At Player`)
      ; frm player
      (bind _asabp_look_at_poi_char (cast `/Game/IsolatedExamples/LookAtPOI/TestLevelContent/Characters/ABP_LookAtPOI_Char` (`self.AnimInstance`)))
      (set `/Game/IsolatedExamples/LookAtPOI/TestLevelContent/Characters/ABP_LookAtPOI_Char.LookAtPOI Target` (`SceneComponent.GetSocketLocation` (`self.GetComponentByClass` (`self.Player Pawn`) "/Script/Engine.SkeletalMeshComponent") "head") _asabp_look_at_poi_char)
      (else
        ; frm gizmo
        (bind _asabp_look_at_poi_char_2 (cast `/Game/IsolatedExamples/LookAtPOI/TestLevelContent/Characters/ABP_LookAtPOI_Char` (`self.AnimInstance`)))
        (set `/Game/IsolatedExamples/LookAtPOI/TestLevelContent/Characters/ABP_LookAtPOI_Char.LookAtPOI Target` (+ (`self.K2_GetActorLocation` _gizmo_obj) (* (`KismetMathLibrary.GetRightVector` (`self.K2_GetActorRotation` _gizmo_obj)) (* _returnvalue_x 50.0))) _asabp_look_at_poi_char_2)))))

(fn `UserConstructionScript`)