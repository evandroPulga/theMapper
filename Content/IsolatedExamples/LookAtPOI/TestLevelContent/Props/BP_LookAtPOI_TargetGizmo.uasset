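; Interactive target gizmo for the LookAtPOI example level that can be rotated and scaled with the mouse.
; Hovering the Hitbox and holding Left Shift takes control, which persists off-hover until Shift is released.
; Tick turns buffered mouse-position deltas into roll and yaw, and wheel input into clamped uniform scale.
; A dynamic material color shows idle, hover or controlled state, while camera-oriented debug text displays control hints.
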(event `self.ReceiveBeginPlay`
  (set `self.Drawer` (`DrawDebugLibrary.MakeDebugDrawer`))
  (`self.SetActorTickInterval` 0.01))

(event `self.ReceiveTick`
  (params (DeltaSeconds :type "Float (single-precision)"))
  (bind _scale_sensetivity (`self.Scale Sensetivity`))
  (bind (_previous_mouse_pos_x _previous_mouse_pos_y) (`KismetMathLibrary.BreakVector2D` (`self.Previous Mouse Pos`)))
  (bind (_locationx _locationy) (`PlayerController.GetMousePosition` (`GameplayStatics.GetPlayerController` 0)))
  (bind _returnvalue (`PlayerController.GetInputAnalogKeyState` (`GameplayStatics.GetPlayerController` 0) "MouseWheelAxis"))
  (bind _returnvalue_2 (`KismetMathLibrary.MapRangeClamped` _returnvalue -10.0 10.0 (* _scale_sensetivity -1.0) _scale_sensetivity))
  (`|ExecutionSequence`
    (:`then_0`
      (if (or (`self.Is Mouse Over`) (`self.Is Controlled`))
        ; Is SHIFT down
        (if (== (`PlayerController.GetInputAnalogKeyState` (`GameplayStatics.GetPlayerController` 0) "LeftShift") 1.0)
          (set `self.Is Controlled` true)
          (else
            (set `self.Is Controlled` false)))))
    (:`then_1`
      (`self.Set Parallel To Camera & Show Tooltip`)
      (`self.Set Color`))
    (:`then_2`
      ; Rotate w/ Mouse
      (if (`self.Is Controlled`)
        (`self.K2_SetActorRotation` self (`KismetMathLibrary.MakeRotator` (`KismetMathLibrary.ClampAxis` (+ (.roll (`self.K2_GetActorRotation` self)) (* (- _previous_mouse_pos_y _locationy) -1.0))) 0.0 (`KismetMathLibrary.ClampAxis` (+ (.yaw (`self.K2_GetActorRotation` self)) (- _previous_mouse_pos_x _locationx)))) false)
        ; Scale w/ Mouse Wheel
        (if (not (`KismetMathLibrary.NearlyEqual_FloatFloat` _returnvalue))
          (`self.SetActorScale3D` self (`KismetMathLibrary.ClampVectorSize` (+ (.scale (`self.GetTransform` self)) (`KismetMathLibrary.MakeVector` _returnvalue_2 _returnvalue_2 _returnvalue_2)) 0.3 20.0)))))
    (:`then_4`
      (`self.Buffer Mouse Pos`))))

(event `self.hitbox.OnBeginCursorOver`
  (params (TouchedComponent :type "PrimitiveComponent Object Reference"))
  (set `self.Is Mouse Over` true))

(event `self.hitbox.OnEndCursorOver`
  (params (TouchedComponent :type "PrimitiveComponent Object Reference"))
  (set `self.Is Mouse Over` false))

(fn `Buffer Mouse Pos`
  (bind (_locationx _locationy) (`PlayerController.GetMousePosition` (`GameplayStatics.GetPlayerController` 0)))
  (set `self.Previous Mouse Pos` (`KismetMathLibrary.MakeVector2D` _locationx _locationy)))

(fn `Set Color`
  (`MaterialInstanceDynamic.SetVectorParameterValue` (`self.Border Dynamic Material`) "Diffuse" (select `bool` (`self.Is Controlled`) :`false` (select `bool` (`self.Is Mouse Over`) :`false` (`self.Color Gray`) :`true` (`self.Color White`)) :`true` (`self.Color Green`))))

(fn `Set Parallel To Camera & Show Tooltip`
  (bind (_returnvalue_roll _returnvalue_pitch _returnvalue_yaw) (`KismetMathLibrary.BreakRotator` (`PlayerCameraManager.GetCameraRotation` (`GameplayStatics.GetPlayerCameraManager` 0))))
  (if (or (`self.Is Mouse Over`) (`self.Is Controlled`))
    (`DrawDebugLibrary.DrawDebugText` (`self.Drawer`) (`KismetMathLibrary.SelectText` "Rotate by moving Mouse \nScale with Mouse Wheel" "Hold L Shift Down" (`self.Is Controlled`)) (+ (* (.location (`self.GetTransform`)) (1.0 1.0 0.0)) (0.0 0.0 300.0)) (`KismetMathLibrary.ComposeRotators` (`KismetMathLibrary.MakeRotator` _returnvalue_roll 0.0 _returnvalue_yaw)) (make `DrawDebugLineStyle` (struct :`R` 1.0 :`G` 1.0 :`B` 1.0 :`A` 1.0) 1.0) false (make `DrawDebugStringSettings` (`KismetMathLibrary.SelectFloat` 12.0 18.0 (`self.Is Controlled`))))))

(fn `UserConstructionScript`
  (bind _returnvalue (`PrimitiveComponent.CreateDynamicMaterialInstance` (`self.geo`) 0 null "None"))
  (set `self.Border Dynamic Material` _returnvalue)
  (`PrimitiveComponent.SetMaterial` (`self.geo`) 0 (`self.Border Dynamic Material`))
  (`MaterialInstanceDynamic.SetVectorParameterValue` (`self.Border Dynamic Material`) "Diffuse" (`self.Color Gray`)))