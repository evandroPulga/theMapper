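; Selectable zone border for the LookAtPOI test level, tied to an assigned pawn.
; Construction sizes outline meshes, label and hitbox and caches world bounds; dynamic materials show hover and selection.
; Clicking deselects other zones, disabling their pawns' look-at, spawns a target gizmo unless the controller's LookAtPlayer is set, and notifies PC_LookAtPOI.
; Tick keeps the gizmo offset from the pawn, orients the label to the camera and draws the hover tooltip.
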(event `self.ReceiveBeginPlay`
  (`|ExecutionSequence`
    (:`then_0`
      ; Bind Mouse Events
      (for _array_element (`self.Meshes For Mouse Over`)
        (add `PrimitiveComponent.OnBeginCursorOver` _array_element (`|CreateDelegate` :!event `On Begin Mouse Over`))
        (add `PrimitiveComponent.OnEndCursorOver` _array_element (`|CreateDelegate` :!event `On End Mouse Over`))
        (add `PrimitiveComponent.OnClicked` _array_element (`|CreateDelegate` :!event `On Mouse Clicked`))))
    (:`then_1`
      ; Collect all instanses
      (`KismetSystemLibrary.Delay` 0.5)
      (bind _outactors (`GameplayStatics.GetAllActorsOfClass` "BP_LookAtPOI_BorderObj_C"))
      (set `self.All Bodred Objects` _outactors))))

(event `self.ReceiveTick`
  (params (DeltaSeconds :type "Float (single-precision)"))
  (`self.Set Parallel To Camera & Show Tooltip`)
  (bind _gizmo_obj (`self.Gizmo Obj`)
    (:`then`
      (`self.K2_SetActorLocation` _gizmo_obj (`self.Get Gizmo Pos`) false false))
    (:`else`)))

(event `On Begin Mouse Over`
  (params (TouchedComponent :type "PrimitiveComponent Object Reference"))
  ;[1 1 1] Highlight Material On Mesh Hover
  (`MaterialInstanceDynamic.SetVectorParameterValue` (`self.Border Dynamic Material`) "Diffuse" (struct :`R` 1.0 :`G` 1.0 :`B` 1.0 :`A` 1.0))
  (`MaterialInstanceDynamic.SetVectorParameterValue` (`self.Text Dynamic Material`) "Diffuse" (struct :`R` 1.0 :`G` 1.0 :`B` 1.0 :`A` 1.0))
  (set `self.Is Mouse Over` true) ; Store hovered state
)

(event `On End Mouse Over`
  (params (TouchedComponent :type "PrimitiveComponent Object Reference"))
  (bind _returnvalue (select `bool` (`self.Is Selected`) :`false` (`self.Color Gray`) :`true` (`self.Color Green`)))
  ;[1 1 1] Highlight Material On Mesh Hover
  (set `self.Is Mouse Over` false)
  (`MaterialInstanceDynamic.SetVectorParameterValue` (`self.Border Dynamic Material`) "Diffuse" _returnvalue :!label _label)
  (`MaterialInstanceDynamic.SetVectorParameterValue` (`self.Text Dynamic Material`) "Diffuse" _returnvalue))

(event `Set Color`
  (goto _label))

(event `On Mouse Clicked`
  (params (TouchedComponent :type "PrimitiveComponent Object Reference") (ButtonPressed :type "Key Structure" :default "None"))
  (`self.Gizmo Obj`
    (:`then`)
    (:`else`
      (`|ExecutionSequence`
        (:`then_0`
          ; Comment
          (`self.Dispatch On Mouse Clicked`)
          (set `self.Is Selected` true)
          (`self.Set Color`))
        (:`then_1`
          ; Spawn Gizmo Object
          (`self.Controller Looks At Gizmo`
            (:`True`
              (bind _returnvalue (`|SpawnActorFromClass` "/Game/IsolatedExamples/LookAtPOI/TestLevelContent/Props/BP_LookAtPOI_TargetGizmo.BP_LookAtPOI_TargetGizmo_C" (`KismetMathLibrary.MakeTransform` (`self.Get Gizmo Pos`) (`self.K2_GetActorRotation`)) "Undefined" "MultiplyWithRoot" null null))
              (bind _output_get (set `self.Gizmo Obj` _returnvalue))
              (`self.SetActorScale3D` _output_get (`KismetMathLibrary.Conv_DoubleToVector` 4.0)))))
        (:`then_2`
          ; Clear all other zone objects
          (for _array_element (`self.All Bodred Objects`)
            (if (!= _array_element self)
              (`self.Deselect Zone` _array_element))))
        (:`then_3`
          ; Set selected pawn onto a controller
          (bind _aspc_look_at_poi (cast `/Game/IsolatedExamples/LookAtPOI/TestLevelContent/Controllers/PC_LookAtPOI` (`GameplayStatics.GetPlayerController` 0)))
          (`/Game/IsolatedExamples/LookAtPOI/TestLevelContent/Controllers/PC_LookAtPOI.Zone Was Selected` _aspc_look_at_poi (`self.Assigned Pawn`) (`self.Zone Type`) (`self.Gizmo Obj`)))))))

(event `Deselect Zone`
  ; Deselect Zone
  (set `self.Is Selected` false)
  (`self.Set Color`)
  (`|ExecutionSequence`
    (:`then_0`
      (bind _gizmo_obj (`self.Gizmo Obj`)
        (:`then`
          (`self.K2_DestroyActor` _gizmo_obj)
          (set `self.Gizmo Obj` null))
        (:`else`)))
    (:`then_1`
      (bind _aspawn_look_at_poi_char (`self.Validate Get LookAtPOI Pawn`))
      (set `/Game/IsolatedExamples/LookAtPOI/TestLevelContent/Characters/Pawn_LookAt_POI_Char.LookAtPOI Enabled` false _aspawn_look_at_poi_char))))

(event `Update Border`
  ; Update border
  (`self.Init Text Label`)
  (`self.Init Outline Mesh` (`self.Volume Width`) (`self.Volume Length`))
  (`self.Set Zone Limits`))

(fn `Get Gizmo Pos`
  (returns (ReturnValue :type "Vector Structure"))
  (return (+ (`self.K2_GetActorLocation` (`self.Assigned Pawn`)) (`self.Gizmo Offset`))))

(fn `Init Outline Mesh`
  (params (`Volume Width` :type "Float (double-precision)") (`Volume Length` :type "Float (double-precision)"))
  (locals (Width :type "Float (double-precision)") (Length :type "Float (double-precision)"))
  (bind _width (`local.Width`))
  (bind _length (`local.Length`))
  (bind _length_2 (`local.Length`))
  (bind _width_2 (`local.Width`))
  (bind _array (`|MakeArray` (`self.Corner_Lt_Top`) (`self.Corner_Rt_Bot`) (`self.Corner_Rt_Top`) (`self.Line Bottom`) (`self.Line Left`) (`self.Line Right`) (`self.Line Top`) (`self.Corner_Lt_Bot`)))
  (bind _returnvalue (* _length_2 -1.0))
  (bind _returnvalue_2 (* _width_2 -1.0))
  (bind _returnvalue_3 (/ (- (`local.Width`) 100.0) 100.0))
  (bind _returnvalue_4 (/ (- (`local.Length`) 100.0) 100.0))
  (set `local.Width` `Volume Width`)
  (set `local.Length` `Volume Length`)
  (`|ExecutionSequence`
    (:`then_0`
      ;[1 1 1] Form Green outline volume
      (`|ExecutionSequence`
        (:`then_0`
          (`SceneComponent.K2_SetRelativeTransform` (`self.Line Left`) (`KismetMathLibrary.MakeTransform` (`KismetMathLibrary.MakeVector` 0.0 (* _width -1.0)) (struct) (`KismetMathLibrary.MakeVector` _returnvalue_4 1.0 1.0)) false false)
          (`SceneComponent.K2_SetRelativeTransform` (`self.Line Right`) (`KismetMathLibrary.MakeTransform` (`KismetMathLibrary.MakeVector` 0.0 _width) (struct :`Yaw` 180.0) (`KismetMathLibrary.MakeVector` _returnvalue_4 1.0 1.0)) false false))
        (:`then_1`
          (`SceneComponent.K2_SetRelativeTransform` (`self.Line Top`) (`KismetMathLibrary.MakeTransform` (`KismetMathLibrary.MakeVector` _length) (struct :`Yaw` 90.0) (`KismetMathLibrary.MakeVector` _returnvalue_3 1.0 1.0)) false false)
          (`SceneComponent.K2_SetRelativeTransform` (`self.Line Bottom`) (`KismetMathLibrary.MakeTransform` (`KismetMathLibrary.MakeVector` (* _length -1.0)) (struct :`Yaw` -90.0) (`KismetMathLibrary.MakeVector` _returnvalue_3 1.0 1.0)) false false))
        (:`then_2`
          (`SceneComponent.K2_SetRelativeTransform` (`self.Corner_Lt_Bot`) (`KismetMathLibrary.MakeTransform` (`KismetMathLibrary.MakeVector` _returnvalue _returnvalue_2) (struct) (1.0 1.0 1.0)) false false)
          (`SceneComponent.K2_SetRelativeTransform` (`self.Corner_Lt_Top`) (`KismetMathLibrary.MakeTransform` (`KismetMathLibrary.MakeVector` _length_2 _returnvalue_2) (struct) (-1.0 1.0 1.0)) false false)
          (`SceneComponent.K2_SetRelativeTransform` (`self.Corner_Rt_Bot`) (`KismetMathLibrary.MakeTransform` (`KismetMathLibrary.MakeVector` _returnvalue _width_2) (struct) (1.0 -1.0 1.0)) false false)
          (`SceneComponent.K2_SetRelativeTransform` (`self.Corner_Rt_Top`) (`KismetMathLibrary.MakeTransform` (`KismetMathLibrary.MakeVector` _length_2 _width_2) (struct) (-1.0 -1.0 1.0)) false false))))
    (:`then_1`
      ;[1 1 1] Store Material
      (bind _returnvalue_5 (`PrimitiveComponent.CreateDynamicMaterialInstance` (`self.Corner_Lt_Bot`) 0 null "None"))
      (set `self.Border Dynamic Material` _returnvalue_5))
    (:`then_2`
      ;[1 1 1] Set Material
      (`KismetArrayLibrary.Array_Append` (`self.Meshes For Mouse Over`) _array)
      (for _array_element _array
        (`PrimitiveComponent.SetMaterial` _array_element 0 (`self.Border Dynamic Material`))
        (`MaterialInstanceDynamic.SetVectorParameterValue` (`self.Border Dynamic Material`) "Diffuse" (`self.Color Gray`))))))

(fn `Init Text Label`
  (bind _text_render_obj (`self.Text Render Obj`))
  (bind _mesh_hitboxformouse (`self.Mesh HitboxForMouse`))
  (bind (_returnvalue_x _returnvalue_y _returnvalue_z) (`KismetMathLibrary.BreakVector` (`TextRenderComponent.GetTextLocalSize` (`self.Text Render Obj`))))
  (`|ExecutionSequence`
    (:`then_0`
      (`TextRenderComponent.K2_SetText` (`self.Text Render Obj`) (`self.Zone Name`)))
    (:`then_1`
      ;[1 1 1] Set Hitbox To Text Size
      (`SceneComponent.K2_SetRelativeLocation` _mesh_hitboxformouse (`KismetMathLibrary.MakeVector` 0.0 (/ _returnvalue_y -2.0)) false false)
      (`SceneComponent.SetRelativeScale3D` _mesh_hitboxformouse (`KismetMathLibrary.MakeVector` (`KismetMathLibrary.FMax` (/ _returnvalue_x 100.0) 0.01) (`KismetMathLibrary.FMax` (/ _returnvalue_y 100.0) 0.01) (`KismetMathLibrary.FMax` (/ _returnvalue_z 100.0) 0.01))))
    (:`then_2`
      ;[1 1 1] Assign Dynamic Material
      (bind _returnvalue (`PrimitiveComponent.CreateDynamicMaterialInstance` _text_render_obj 0 null "None"))
      (bind _output_get (set `self.Text Dynamic Material` _returnvalue))
      (`PrimitiveComponent.SetMaterial` _text_render_obj 0 _output_get)
      (`MaterialInstanceDynamic.SetVectorParameterValue` _output_get "Diffuse" (`self.Color Gray`)))
    (:`then_3`
      ; Add mesh hitbox
      (`KismetArrayLibrary.Array_Add` (`self.Meshes For Mouse Over`) (`self.Mesh HitboxForMouse`)))))

(fn `Set Look At Target`
  (params (`Look At POI Pawn` :type "/Game/IsolatedExamples/LookAtPOI/TestLevelContent/Characters/Pawn_LookAt_POI_Char Object Reference"))
  (bind _gizmo_obj (`self.Gizmo Obj`))
  (bind _returnvalue_x (`KismetMathLibrary.BreakVector` (`self.GetActorScale3D` _gizmo_obj)))
  (set `/Game/IsolatedExamples/LookAtPOI/TestLevelContent/Characters/Pawn_LookAt_POI_Char.LookAtPOI Target` (+ (`self.K2_GetActorLocation` _gizmo_obj) (* (`KismetMathLibrary.GetRightVector` (`self.K2_GetActorRotation` _gizmo_obj)) (* _returnvalue_x 50.0))) `Look At POI Pawn`))

(fn `Set Parallel To Camera & Show Tooltip`
  (bind _returnvalue (`GameplayStatics.GetPlayerCameraManager` 0))
  (bind (_returnvalue_roll _returnvalue_pitch _returnvalue_yaw) (`KismetMathLibrary.BreakRotator` (`PlayerCameraManager.GetCameraRotation` _returnvalue)))
  (`/Engine/EditorBlueprintResources/StandardMacros.IsValid` _returnvalue
    (:`Is Valid`
      (`SceneComponent.K2_SetWorldRotation` (`self.Text Render Obj`) (`KismetMathLibrary.ComposeRotators` (`KismetMathLibrary.MakeRotator` _returnvalue_roll 0.0 _returnvalue_yaw) (struct :`Yaw` 180.0)) false false)
      (if (and (`self.Is Mouse Over`) (not (`self.Is Selected`)))
        (`DrawDebugLibrary.DrawDebugText` (`DrawDebugLibrary.MakeDebugDrawer`) "Click to Select" (`SceneComponent.K2_GetComponentLocation` (`self.Text Render Obj`)) (`KismetMathLibrary.ComposeRotators` (`KismetMathLibrary.MakeRotator` _returnvalue_roll 0.0 _returnvalue_yaw)) (make `DrawDebugLineStyle` (struct :`R` 1.0 :`G` 1.0 :`B` 1.0 :`A` 1.0) 1.0) false (make `DrawDebugStringSettings` 22.0))))))

(fn `Set Zone Limits`
  (bind (_returnvalue_x _returnvalue_y) (`KismetMathLibrary.BreakVector` (`SceneComponent.K2_GetComponentLocation` (`self.Corner_Rt_Bot`))))
  (bind (_returnvalue_x_2 _returnvalue_y_2) (`KismetMathLibrary.BreakVector` (`SceneComponent.K2_GetComponentLocation` (`self.Corner_Lt_Bot`))))
  (bind (_returnvalue_x_3 _returnvalue_y_3) (`KismetMathLibrary.BreakVector` (`SceneComponent.K2_GetComponentLocation` (`self.Corner_Rt_Top`))))
  (bind (_returnvalue_x_4 _returnvalue_y_4) (`KismetMathLibrary.BreakVector` (`SceneComponent.K2_GetComponentLocation` (`self.Corner_Lt_Top`))))
  (set `self.Zone Limits X` (`KismetMathLibrary.MakeVector2D` (`KismetMathLibrary.FMin` _returnvalue_x_4 _returnvalue_x _returnvalue_x_3 _returnvalue_x_2) (`KismetMathLibrary.FMax` _returnvalue_x_4 _returnvalue_x _returnvalue_x_3 _returnvalue_x_2)))
  (set `self.Zone Limits Y` (`KismetMathLibrary.MakeVector2D` (`KismetMathLibrary.FMin` _returnvalue_y_4 _returnvalue_y _returnvalue_y_3 _returnvalue_y_2) (`KismetMathLibrary.FMax` _returnvalue_y_4 _returnvalue_y _returnvalue_y_3 _returnvalue_y_2))))

(fn `UserConstructionScript`
  (`self.Init Text Label`)
  (`self.Init Outline Mesh` (`self.Volume Width`) (`self.Volume Length`))
  (`self.Set Zone Limits`))