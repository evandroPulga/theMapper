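; Mover movement mode for ragdolling characters that makes the capsule follow the ragdoll transform supplied through custom inputs.
; A downward sphere trace adjusts the target height when ground is hit, with debug drawing toggled by a console variable.
; The capsule safe-moves and slides to the target, rotating toward orientation intent.
; It derives linear and angular velocity from that change and writes them with the resulting transform to the sync state.
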(event `self.K2_OnActivated`)

(fn `SimulationTick`
  (params (Params :type "SimulationTickParams Structure (by ref)") (OutputState :type "MoverTickEndData Structure (by ref)"))
  (locals (MoverDefaultInputs :type "CharacterDefaultInputs Structure") (CustomInputs_Ragdoll :type "/Game/Blueprints/Data/S_MoverCustomInputs_Ragdoll Structure") (DefaultSyncState :type "MoverDefaultSyncState Structure") (OutHit :type "HitResult Structure") (TargetCapsuleTransform :type "Transform Structure") (MoveDelta :type "Vector Structure") (Velocity :type "Vector Structure") (AngularVelocity :type "Vector Structure") (DebugState :type Integer))
  (bind _targetcapsuletransform_location (`KismetMathLibrary.BreakTransform` (`local.TargetCapsuleTransform`)))
  (bind _custominputs_ragdoll_ragdolltransform (break `/Game/Blueprints/Data/S_MoverCustomInputs_Ragdoll` (`local.CustomInputs_Ragdoll`)))
  (bind _custominputs_ragdoll (`local.CustomInputs_Ragdoll`))
  (bind (_remainingms _nextmodename _bendedwithnochanges) (break `MovementModeTickEndState` (`.MovementEndState` (break `MoverTickEndData` (`local.OutputState`)))))
  (bind ((`UpdatedComponent` _updatedcomponent)) (break `MovingComponentSet` (`.MovingComps` (break `SimulationTickParams` (`local.Params`)))))
  (bind _inputcollection (break `MoverInputCmdContext` (`.InputCmd` (break `MoverTickStartData` (`.StartState` (break `SimulationTickParams` (`local.Params`)))))))
  (`|ExecutionSequence`
    (:`then_0`
      (bind (_didsucceed _targetasrawbytes) (`MoverDataCollectionLibrary.K2_GetDataFromCollection` _inputcollection))
      (if _didsucceed
        (set `local.CustomInputs_Ragdoll` _targetasrawbytes)
        (bind (_didsucceed_2 _targetasrawbytes_2) (`MoverDataCollectionLibrary.K2_GetDataFromCollection` _inputcollection))
        (set `local.MoverDefaultInputs` _targetasrawbytes_2)
        (bind _returnvalue (`KismetSystemLibrary.GetConsoleVariableIntValue` "DDCVar.CharacterPhysics.DrawDebug"))
        (set `local.DebugState` _returnvalue)))
    (:`then_1`
      (bind _output_get (set `local.TargetCapsuleTransform` _custominputs_ragdoll_ragdolltransform))
      (bind _outhit (`KismetSystemLibrary.SphereTraceSingle` :`Start` (.location _output_get) :`End` (`KismetMathLibrary.MakeVector` (.x (.location _output_get)) (.y (.location _output_get)) (- (.z (.location _output_get)) 88.0)) :`Radius` 30.0 :`TraceChannel` "TraceTypeQuery1" :`DrawDebugType` (select `int` (`local.DebugState`) :`0` "None" :`1` "ForOneFrame" :!type "EDrawDebugTrace Enum")))
      (if (`GameplayStatics.BreakHitResult` _outhit)
        (set `local.TargetCapsuleTransform` (`KismetMathLibrary.MakeTransform` (`KismetMathLibrary.MakeVector` (.x (.location (break `/Game/Blueprints/Data/S_MoverCustomInputs_Ragdoll` _custominputs_ragdoll))) (.y (.location (break `/Game/Blueprints/Data/S_MoverCustomInputs_Ragdoll` _custominputs_ragdoll))) (+ (.z (.location (break `/Game/Blueprints/Data/S_MoverCustomInputs_Ragdoll` _custominputs_ragdoll))) (- 86.0 (`KismetMathLibrary.Abs` (- (.z (`.ImpactPoint` (`GameplayStatics.BreakHitResult` _outhit))) (.z (`.TraceStart` (`GameplayStatics.BreakHitResult` _outhit)))))) 1.9)) (.rotation (break `/Game/Blueprints/Data/S_MoverCustomInputs_Ragdoll` _custominputs_ragdoll)) (.scale (break `/Game/Blueprints/Data/S_MoverCustomInputs_Ragdoll` _custominputs_ragdoll))))))
    (:`then_2`
      (bind (_didsucceed_3 _targetasrawbytes_3) (`MoverDataCollectionLibrary.K2_GetDataFromCollection` (`.SyncStateCollection` (break `MoverSyncState` (`.SyncState` (break `MoverTickStartData` (`.StartState` (break `SimulationTickParams` (`local.Params`)))))))))
      (bind _output_get_2 (set `local.DefaultSyncState` _targetasrawbytes_3))
      (bind _returnvalue_2 (`MoverDataModelBlueprintLibrary.GetLocationFromSyncState` _output_get_2))
      (set `local.MoveDelta` (- _targetcapsuletransform_location _returnvalue_2))
      (`MovementUtils.TrySafeMoveAndSlideUpdatedComponentNoMovementRecord` (`.MovingComps` (break `SimulationTickParams` (`local.Params`))) (`local.MoveDelta`) (`KismetMathLibrary.Conv_RotatorToQuaternion` (`KismetMathLibrary.Conv_VectorToRotator` (`.OrientationIntent` (break `CharacterDefaultInputs` (`local.MoverDefaultInputs`))))) false (`local.OutHit`))
      (set `local.Velocity` (/ (`local.MoveDelta`) (* (`.StepMs` (break `MoverTimeStep` (`.TimeStep` (break `SimulationTickParams` (`local.Params`))))) 0.001)))
      (bind _returnvalue_3 (`MoverDataModelBlueprintLibrary.GetOrientationFromSyncState` (`local.DefaultSyncState`)))
      (bind _returnvalue_4 (`MovementUtils.ComputeAngularVelocityDegrees` _returnvalue_3 (`KismetMathLibrary.Conv_VectorToRotator` (`.OrientationIntent` (break `CharacterDefaultInputs` (`local.MoverDefaultInputs`)))) (* (`.StepMs` (break `MoverTimeStep` (`.TimeStep` (break `SimulationTickParams` (`local.Params`))))) 0.001)))
      (set `local.AngularVelocity` _returnvalue_4))
    (:`then_3`
      (`MoverDataCollectionLibrary.K2_AddDataToCollection` (`.SyncStateCollection` (break `MoverSyncState` (`.SyncState` (break `MoverTickEndData` (`local.OutputState`))))) (make `MoverDefaultSyncState` :`Location` (`SceneComponent.K2_GetComponentLocation` _updatedcomponent) :`Orientation` (`SceneComponent.K2_GetComponentRotation` _updatedcomponent) :`Velocity` (`local.Velocity`) :`AngularVelocityDegrees` (`local.AngularVelocity`)))
      (setmembers `MoverTickEndData` :`StructRef` (`local.OutputState`) :`MovementEndState` (make `MovementModeTickEndState` 0.0 _nextmodename _bendedwithnochanges))
      (return))))